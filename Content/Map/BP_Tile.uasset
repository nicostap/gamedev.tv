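; BP_Tile is a map tile Blueprint that randomizes which of its 24 numbered components are shown.
; Its Construction Script loops over those components and gives each a one-in-three chance of being set visible.
; It never hides a component, so unselected ones keep their default visibility.
; The event graph holds only disabled placeholder events, so the tile has no runtime logic there.
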(event EventBeginPlay)

(event Collision|EventActorBeginOverlap
  (params (OtherActor :type Actor%20Object%20Reference)))

(event EventTick
  (params (DeltaSeconds :type Float%20%28single-precision%29)))

(fn ConstructionScript
  (bind _output_get (Variables|Default|SetArrry (Utilities|Array|MakeArray (Variables|Default|Get1) (Variables|Default|Get2) (Variables|Default|Get3) (Variables|Default|Get4) (Variables|Default|Get5) (Variables|Default|Get6) (Variables|Default|Get7) (Variables|Default|Get8) (Variables|Default|Get9) (Variables|Default|Get10) (Variables|Default|Get11) (Variables|Default|Get12) (Variables|Default|Get13) (Variables|Default|Get14) (Variables|Default|Get15) (Variables|Default|Get16) (Variables|Default|Get17) (Variables|Default|Get18) (Variables|Default|Get19) (Variables|Default|Get20) (Variables|Default|Get21) (Variables|Default|Get22) (Variables|Default|Get23) (Variables|Default|Get24))))
  (for _array_element _output_get
    (if (== (Math|Random|RandomInteger 3) 2)
      (Rendering|SetVisibility _array_element true false))))